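; BP_Test08_Enemy is a test enemy character that repeatedly swings a hatchet axe and ragdolls when it dies.
; On BeginPlay it spawns, initializes and equips its weapon, attacks, and starts a looping timer, apparently to repeat the attack.
; Attack chains three montage combo sections, each starting when the previous completes.
; StatComponent's death event stops the montage and timer, then switches the mesh to physics ragdoll.
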(event Custom|OnDie
  (Animation|StopAnimMontage (Animation|GetCurrentMontage :!class /Script/Engine.Character))
  (Utilities|Time|ClearandInvalidateTimerbyHandle (Variables|Default|GetAttackTimerHandle))
  (Collision|SetCollisionProfileName (Variables|Character|GetMesh) "Ragdoll" true :!class /Script/Engine.PrimitiveComponent)
  (Class|SkeletalMeshComponent|SetAllBodiesSimulatePhysics (Variables|Character|GetMesh) true)
  (Collision|SetCollisionObjectType (Variables|Character|GetMesh) "ECC_PhysicsBody")
  (Components|SkeletalMesh|SetAnimInstanceClass (Variables|Character|GetMesh) 0))

(event Custom|Attack
  (Animation|Montage|PlayMontage (Variables|Character|GetMesh) (Variables|Default|GetAttackMontage) 1.0 0.0 "Combo1"
    (:OnCompleted
      (Animation|Montage|PlayMontage (Variables|Character|GetMesh) (Variables|Default|GetAttackMontage) 1.0 0.0 "Combo2"
        (:OnCompleted
          (Animation|Montage|PlayMontage (Variables|Character|GetMesh) (Variables|Default|GetAttackMontage) 1.0 0.0 "Combo3"))))))

(event EventBeginPlay
  (EventDispatchers|BindEventtoOnDie (Variables|Default|GetStatComponent) (EventDispatchers|CreateEvent :!event Custom|OnDie))
  (bind _returnvalue (Game|SpawnActorfromClass "/Game/Blueprints/_TEST/Test08/BP_Test08_EnemyWeapon.BP_Test08_EnemyWeapon_C" (Math|Transform|MakeTransform "0, 0, 0" "0, 0, 0" "1.000000,1.000000,1.000000") "Undefined" "MultiplyWithRoot" 0 self))
  (Class|WeaponActor|InitializeWeapon _returnvalue "/Game/Data/Item/Weapon/DA_Weapon_HatchetAxe.DA_Weapon_HatchetAxe")
  (Class|WeaponActor|OnEquipped _returnvalue self)
  (CallFunction|Attack)
  (bind _returnvalue_2 (Utilities|Time|SetTimerbyEvent (EventDispatchers|CreateEvent :!event Custom|Attack) 6.0 true))
  (Variables|Default|SetAttackTimerHandle _returnvalue_2))

(fn ConstructionScript)