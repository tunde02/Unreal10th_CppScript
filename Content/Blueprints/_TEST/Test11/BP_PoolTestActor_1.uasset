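; BP_PoolTestActor_1 is a test actor with a Sphere component for use with an object pool.
; Its OnSpawn event shows the actor and enables collision and tick, and OnReturn reverses all three so the instance can sit idle for reuse.
; Physics toggling on the Sphere and a delayed self-return through ObjectPoolSubsystem are present but unconnected, so they never run.
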(event EventOnSpawn
  (Rendering|SetActorHiddenInGame false)
  (Collision|SetActorEnableCollision true)
  (Actor|Tick|SetActorTickEnabled true))

(event EventOnReturn
  (Rendering|SetActorHiddenInGame true)
  (Collision|SetActorEnableCollision false)
  (Actor|Tick|SetActorTickEnabled false))

(fn ConstructionScript)