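; BP_PoolTestActor_2 is a test actor for an object pooling system, built around a Cube component.
; OnSpawn turns on physics simulation for the cube, while OnReturn is empty.
; Disconnected nodes, which never run, hold manual show and hide logic for transform, visibility, collision and tick, plus a delayed return to the ObjectPoolSubsystem.
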(event EventOnSpawn
  (Physics|SetSimulatePhysics (Variables|Default|GetCube) true))

(event EventOnReturn)

(fn ConstructionScript)